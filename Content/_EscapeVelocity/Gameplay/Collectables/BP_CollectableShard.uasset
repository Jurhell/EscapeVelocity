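; Collectable shard pickup that adds its ScoreValue to the player's Score when a BP_Player overlaps it.
; On pickup it moves the Niagara effect to the box's transform at unit scale and activates it.
; It then shrinks the root to near zero rather than destroying immediately, and destroys the actor after a short delay.
; The construction script copies RotateToGravity into CorrectRotation before running the parent's construction.
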(event Collision|EventActorBeginOverlap
  (params (OtherActor :type Actor%20Object%20Reference))
  (bind _box (Variables|Default|GetBox))
  (bind _niagara (Variables|Default|GetNiagara))
  (bind _returnvalue (Transformation|GetWorldTransform _box))
  (|CallParentFunction OtherActor)
  (bind _asbp_player (Utilities|Casting|CastToBP_Player OtherActor))
  (Variables|/Game/_EscapeVelocity/Characters/Player/BP_Player.BP_Player_C|SetScore _asbp_player (+ (Variables|/Game/_EscapeVelocity/Characters/Player/BP_Player.BP_Player_C|GetScore _asbp_player) (Variables|Default|GetScoreValue)))
  ;[0.01764 0.01764 0.01764] Play vfx
  (|SetVFXTransform _niagara (.location _returnvalue) (.rotation _returnvalue))
  (Components|Activation|Activate _niagara false)
  ;[0.01764 0.01764 0.01764] Destroy actor
  (Transformation|SetWorldScale3D (Variables|Default|GetDefaultSceneRoot) "0.001000,0.001000,0.001000")
  (Utilities|FlowControl|Delay 2.0)
  (Actor|DestroyActor))

(event EventBeginPlay
  (|CallParentFunction))

(fn ConstructionScript
  (Variables|Default|SetCorrectRotation (Variables|Default|GetRotateToGravity))
  (|CallParentFunction))