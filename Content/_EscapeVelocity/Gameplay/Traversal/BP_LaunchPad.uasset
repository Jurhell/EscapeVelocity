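; BP_LaunchPad is a traversal actor that launches the player when they overlap it.
; On overlap with BP_Player, it stops the character's movement, then launches it along the normalized Direction, rotated by the pad's rotation and scaled by Strength.
; The launch is additive (no XY or Z override), so the preceding stop clears prior momentum.
; Its construction script copies RotateToGravity into CorrectRotation before running the parent's construction script.
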(event EventBeginPlay
  (|CallParentFunction))

(event Collision|EventActorBeginOverlap
  (params (OtherActor :type Actor%20Object%20Reference))
  (bind _asbp_player (Utilities|Casting|CastToBP_Player OtherActor))
  (Components|Movement|StopMovementImmediately (Variables|/Script/Engine.Character|GetCharacterMovement _asbp_player))
  (Character|LaunchCharacter _asbp_player (* (Variables|Default|GetStrength) (Math|Vector|RotateVector (Math|Vector|Normalize (Variables|Default|GetDirection)) (Transformation|GetActorRotation))) false false))

(fn ConstructionScript
  (Variables|Default|SetCorrectRotation (Variables|Default|GetRotateToGravity))
  (|CallParentFunction))