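; Physics object that falls toward nearby gravity platforms rather than along a single world direction.
; Overlap events track gravity sources, and each tick it selects the primary one by mesh surface distance.
; Pull direction is inverted actor up for fixed platforms, or toward the closest collision point for sphere and mesh platforms.
; Tick applies a mass-scaled force, with strength calculated by the player pawn's GetGravityStrength.
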(event Collision|EventActorBeginOverlap
  (params (OtherActor :type Actor%20Object%20Reference))
  (CallFunction|TryAddtoList OtherActor))

(event EventTick
  (params (DeltaSeconds :type Float%20%28single-precision%29))
  (CallFunction|GetNewPrimaryGravityPlatform)
  (bind _primarygravitysource (Variables|Default|GetPrimaryGravitySource)
    (:then
      (bind _gravitydirection (CallFunction|GetGravityDirection _primarygravitysource))
      (bind _strength (|GravityStrength _primarygravitysource)
        (:then
          (Physics|AddForce (Variables|Default|GetStaticMesh) (* _gravitydirection _strength DeltaSeconds 981.0 (Variables|Default|GetFallSpeed) (Physics|GetMass (Variables|Default|GetStaticMesh))) "None" false))))
    (:else)))

(event Collision|EventActorEndOverlap
  (params (OtherActor :type Actor%20Object%20Reference))
  (CallFunction|TryRemovefromList OtherActor))

(event EventBeginPlay
  (Physics|AddForce (Variables|Default|GetStaticMesh) "0.000000,0.000000,10.000000" "None" false)
  (for _array_element (Collision|GetOverlappingActors "/Script/EscapeVelocity.GravitySource" :!class /Script/Engine.Actor)
    (bind _asgravity_source (Utilities|Casting|CastToGravitySource _array_element))
    (Utilities|Array|Add (Variables|Default|GetAppliedGravitySources) _asgravity_source)))

(fn ConstructionScript)

(fn TryAddtoList
  (params (Overlapping%20Actor :type Actor%20Object%20Reference))
  (bind _appliedgravitysources (Variables|Default|GetAppliedGravitySources))
  (bind _asgravity_source (Utilities|Casting|CastToGravitySource Overlapping%20Actor)
    (:then
      ;[0.01938 0.01938 0.01938] AddToListOfSources
      (if (Utilities|Array|ContainsItem _appliedgravitysources _asgravity_source)
        (return)
        (else
          (Utilities|Array|Add _appliedgravitysources _asgravity_source))))
    (:CastFailed
      (return))))

(fn TryRemovefromList
  (params (OverlappingActor :type Actor%20Object%20Reference))
  (bind _appliedgravitysources (Variables|Default|GetAppliedGravitySources))
  (bind _asgravity_source (Utilities|Casting|CastToGravitySource OverlappingActor)
    (:then
      (if (Utilities|Array|ContainsItem (Variables|Default|GetAppliedGravitySources) _asgravity_source)
        (Utilities|Array|RemoveItem _appliedgravitysources _asgravity_source)
        (bind _primarygravitysource (Variables|Default|GetPrimaryGravitySource) ; Find new Primary if invalid
          (:then
            (if (Utilities|Array|IsNotEmpty _appliedgravitysources) ; Is list not empty?
              (if (== _primarygravitysource _asgravity_source) ; Primary Source removed?
                (CallFunction|GetNewPrimaryGravityPlatform :!label _label))
              (else
                (Variables|Default|SetPrimaryGravitySource 0))))
          (:else
            (goto _label)))))
    (:CastFailed
      _))
  (return))

(fn GetDistancetoPlatform
  (params (Platform :type Gravity%20Source%20Object%20Reference))
  (bind _asbp_sphere_platform (Utilities|Casting|CastToBP_SpherePlatform Platform)
    (:then
      (bind _output_get (LocalVariables|SetMesh (Variables|/Game/_EscapeVelocity/Gameplay/GravityPlatforms/BP_SpherePlatform.BP_SpherePlatform_C|GetMesh _asbp_sphere_platform))))
    (:CastFailed
      (bind _asbp_fixed_platform (Utilities|Casting|CastToBP_FixedPlatform Platform)
        (:then
          (LocalVariables|SetMesh (Variables|/Game/_EscapeVelocity/Gameplay/GravityPlatforms/BP_FixedPlatform.BP_FixedPlatform_C|GetMesh _asbp_fixed_platform)))
        (:CastFailed
          (bind _asbp_mesh_platform (Utilities|Casting|CastToBP_MeshPlatform Platform)
            (:then
              (LocalVariables|SetMesh (Variables|/Game/_EscapeVelocity/Gameplay/GravityPlatforms/BP_MeshPlatform.BP_MeshPlatform_C|GetMesh _asbp_mesh_platform)))
            (:CastFailed
              (return 999999999.0)))))))
  (return (Utilities|GetDistancefromMeshSurface _output_get)))

(fn GetNewPrimaryGravityPlatform
  (for _array_element (Variables|Default|GetAppliedGravitySources)
    ;[0.01938 0.01938 0.01938] CompareSourcesByDistance
    (bind _primarygravitysource (Variables|Default|GetPrimaryGravitySource)
      (:then
        (bind _distancetoplatform (CallFunction|GetDistancetoPlatform _array_element))
        (bind _distancetoplatform_2 (CallFunction|GetDistancetoPlatform _primarygravitysource))
        (if (> _distancetoplatform_2 _distancetoplatform)
          (Variables|Default|SetPrimaryGravitySource _array_element :!label _label)))
      (:else
        (goto _label))))
  (return))

(fn GetGravityDirection
  (params (GravitySource :type Gravity%20Source%20Object%20Reference))
  (bind _returnvalue (Transformation|GetActorLocation))
  (bind _returnvalue_2 (Transformation|GetActorLocation))
  (bind _asbp_fixed_platform (Utilities|Casting|CastToBP_FixedPlatform GravitySource)
    (:then
      (LocalVariables|SetDirection (* (Transformation|GetActorUpVector _asbp_fixed_platform) -1.0)))
    (:CastFailed
      (bind _asbp_sphere_platform (Utilities|Casting|CastToBP_SpherePlatform GravitySource)
        (:then
          (bind _output_get (LocalVariables|SetDirection (Math|Vector|GetUnitDirection(Vector) _returnvalue (.OutPointOnBody (Collision|GetClosestPointonCollision (Variables|/Game/_EscapeVelocity/Gameplay/GravityPlatforms/BP_SpherePlatform.BP_SpherePlatform_C|GetMesh _asbp_sphere_platform) _returnvalue "None"))))))
        (:CastFailed
          (bind _asbp_mesh_platform (Utilities|Casting|CastToBP_MeshPlatform GravitySource)
            (:then
              (LocalVariables|SetDirection (Math|Vector|GetUnitDirection(Vector) _returnvalue_2 (.OutPointOnBody (Collision|GetClosestPointonCollision (Variables|/Game/_EscapeVelocity/Gameplay/GravityPlatforms/BP_MeshPlatform.BP_MeshPlatform_C|GetMesh _asbp_mesh_platform) _returnvalue_2 "None")))))
            (:CastFailed
              _))))))
  (return (Math|Vector|Normalize _output_get)))