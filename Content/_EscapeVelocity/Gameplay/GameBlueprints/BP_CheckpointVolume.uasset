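; BP_CheckpointVolume is a one-time checkpoint trigger that updates where the player respawns.
; On the first overlap by BP_Player, it sets the player's RespawnTransform to its own location and rotation while keeping the player's scale.
; If HasSwitches is set, that same overlap also creates a WBP_SwitchCount widget for the first player controller and adds it to the viewport.
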(event EventBeginPlay
  (Variables|Default|SetCheckpointReached? false))

(event Collision|EventActorBeginOverlap
  (params (OtherActor :type Actor%20Object%20Reference))
  (bind _returnvalue (Transformation|GetActorTransform))
  (bind _asbp_player (Utilities|Casting|CastToBP_Player OtherActor))
  (if (not (Variables|Default|GetCheckpointReached?))
    (Variables|Default|SetCheckpointReached? true)
    ;[0.01938 0.01938 0.01938] Set Transform without altering scale
    (Variables|/Game/_EscapeVelocity/Characters/Player/BP_Player.BP_Player_C|SetRespawnTransform _asbp_player (Math|Transform|MakeTransform (.location _returnvalue) (.rotation _returnvalue) (.scale (Transformation|GetActorTransform _asbp_player))))
    (if (Variables|Default|GetHasSwitches?)
      (bind _returnvalue_2 (UserInterface|CreateWidget "/Game/_EscapeVelocity/UI/WBP_SwitchCount.WBP_SwitchCount_C" (Game|GetPlayerController 0)))
      (UserInterface|Viewport|AddtoViewport _returnvalue_2 0))))

(fn ConstructionScript)