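; Actor that orients itself to the gravity of the nearest platform when its construction script runs with CorrectRotation enabled.
; It nudges itself upward, finds GravitySource actors overlapping its Box, and keeps the one with the closest mesh collision surface.
; Gravity direction depends on platform type: fixed down vector, sphere center, or nearest mesh point.
; A delta quaternion rotates the actor's down axis onto that direction.
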(event EventBeginPlay)

(fn ConstructionScript
  (bind _box (Variables|Default|GetBox))
  (if (Variables|Default|GetCorrectRotation)
    (Transformation|AddActorWorldOffset "0.000000,0.000000,1.000000") ; Nudge Actor for overlap
    (bind _outactors (Collision|ComponentOverlapActors _box (Transformation|GetWorldTransform _box) (Utilities|Array|MakeArray "ObjectTypeQuery1") "/Script/EscapeVelocity.GravitySource"))
    (for _array_element _outactors
      (bind _asgravity_source (Utilities|Casting|CastToGravitySource _array_element))
      (CallFunction|SetClosestGravitySource _asgravity_source))
    (bind _closestgravitysource (Variables|Default|GetClosestGravitySource)
      (:then
        ;[0.01938 0.01938 0.01938] Update Actor Rotation
        (bind _gravitydirection (CallFunction|GetGravityDirection _closestgravitysource))
        (Transformation|SetActorRotation (* (Class|KismetMathLibrary|QuatFindBetweenNormals (* (Transformation|GetActorUpVector) -1.0) _gravitydirection) (Math|Conversions|ToQuaternion(Rotator) (Transformation|GetActorRotation)))))
      (:else))))

(fn GetGravityDirection
  (params (GravitySource :type Gravity%20Source%20Object%20Reference))
  (bind _asbp_fixed_platform (Utilities|Casting|CastToBP_FixedPlatform GravitySource)
    (:then
      (Variables|Default|SetGravityDirection (* (Transformation|GetActorUpVector _asbp_fixed_platform) -1.0)))
    (:CastFailed
      (bind _asbp_sphere_platform (Utilities|Casting|CastToBP_SpherePlatform GravitySource)
        (:then
          (Variables|Default|SetGravityDirection (Math|Vector|GetUnitDirection(Vector) (Transformation|GetActorLocation) (Transformation|GetActorLocation _asbp_sphere_platform))))
        (:CastFailed
          (bind _asbp_mesh_platform (Utilities|Casting|CastToBP_MeshPlatform GravitySource)
            (:then
              (Variables|Default|SetGravityDirection (Math|Vector|GetUnitDirection(Vector) (Transformation|GetActorLocation) (.OutPointOnBody (Collision|GetClosestPointonCollision (Variables|/Game/_EscapeVelocity/Gameplay/GravityPlatforms/BP_MeshPlatform.BP_MeshPlatform_C|GetMesh _asbp_mesh_platform) (Transformation|GetActorLocation) "None")))))
            (:CastFailed
              (Variables|Default|SetGravityDirection "0.000000,0.000000,-1.000000") ; Default
            ))))))
  (return (Variables|Default|GetGravityDirection)))

(fn SetClosestGravitySource
  (params (GravitySource :type Gravity%20Source%20Object%20Reference))
  (bind _closestgravitysource (Variables|Default|GetClosestGravitySource)
    (:then
      ;[0.01938 0.01938 0.01938] Compare and Set Closest Gravity Source
      (bind _distance (CallFunction|GetDistancetoSource _closestgravitysource)) ; Current Source
      (bind _distance_2 (CallFunction|GetDistancetoSource GravitySource)) ; Comparison Source
      (if (< _distance_2 _distance)
        (Variables|Default|SetClosestGravitySource GravitySource)
        (return)
        (else
          _)))
    (:else
      (Variables|Default|SetClosestGravitySource GravitySource)))
  (return))

(fn GetDistancetoSource
  (params (GravitySource :type Gravity%20Source%20Object%20Reference))
  ;[0.01938 0.01938 0.01938] Get Source Mesh
  (bind _asbp_fixed_platform (Utilities|Casting|CastToBP_FixedPlatform GravitySource)
    (:then
      (LocalVariables|SetSourceMesh (Variables|/Game/_EscapeVelocity/Gameplay/GravityPlatforms/BP_FixedPlatform.BP_FixedPlatform_C|GetMesh _asbp_fixed_platform)))
    (:CastFailed
      (bind _asbp_sphere_platform (Utilities|Casting|CastToBP_SpherePlatform GravitySource)
        (:then
          (LocalVariables|SetSourceMesh (Variables|/Game/_EscapeVelocity/Gameplay/GravityPlatforms/BP_SpherePlatform.BP_SpherePlatform_C|GetMesh _asbp_sphere_platform)))
        (:CastFailed
          (bind _asbp_mesh_platform (Utilities|Casting|CastToBP_MeshPlatform GravitySource))
          (LocalVariables|SetSourceMesh (Variables|/Game/_EscapeVelocity/Gameplay/GravityPlatforms/BP_MeshPlatform.BP_MeshPlatform_C|GetMesh _asbp_mesh_platform))))))
  (bind _sourcemesh (LocalVariables|GetSourceMesh)
    (:then
      (bind _distance (CallFunction|GetDistancetoMesh _sourcemesh))
      (return _distance))
    (:else
      (return 999999999.0))))

(fn GetDistancetoMesh
  (params (Mesh :type Mesh%20Component%20Object%20Reference))
  (return (.ReturnValue (Collision|GetClosestPointonCollision Mesh (Transformation|GetActorLocation) "None"))))