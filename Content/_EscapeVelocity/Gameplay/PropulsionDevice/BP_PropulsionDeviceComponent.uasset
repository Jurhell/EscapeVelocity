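; Component for the player's propulsion device, which fires oxygen projectiles and launches the owning BP_Player.
; Charge time sets propulsion strength and a capped charge level, while projectiles spawn along or against the camera's view according to aim direction.
; Launch velocity opposes the shot, scaled down sharply when grounded and held to a minimum when airborne, then a cooldown flag is set.
; An angle check labels the launch's vertical component without altering the velocity.
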(event EventBeginPlay)

(event EventTick
  (params (DeltaSeconds :type Float%20%28single-precision%29)))

(fn GetInverseCameraRotation
  (return (* (Math|Vector|GetForwardVector (Transformation|GetWorldRotation (Actor|GetComponentbyClass (Game|GetPlayerCharacter 0) "/Script/Engine.CameraComponent"))) -1.0)))

(fn SpawnProjectile
  (params (ProjectileSpawnLocation :type Arrow%20Component%20Object%20Reference) (IsAimedForward :type Boolean))
  (LocalVariables|SetForward IsAimedForward)
  (bind _output_get (Variables|Default|SetProjectile%20Spawn%20Location ProjectileSpawnLocation))
  (Transformation|SetWorldRotation _output_get (Transformation|GetWorldRotation (Actor|GetComponentbyClass (Game|GetPlayerCharacter 0) "/Script/Engine.CameraComponent")) false false)
  (if (LocalVariables|GetForward)
    _
    (else
      (bind _inverserotationforward (CallFunction|GetInverseCameraRotation))
      (Transformation|SetWorldRotation (Variables|Default|GetProjectile%20Spawn%20Location) (Math|Conversions|RotationFromXVector _inverserotationforward) false false)))
  (Game|SpawnActorfromClass "/Game/_EscapeVelocity/Gameplay/PropulsionDevice/BP_OxygenProjectile.BP_OxygenProjectile_C" (Transformation|GetWorldTransform (Variables|Default|GetProjectile%20Spawn%20Location)) "AlwaysSpawn" "MultiplyWithRoot" 0 0))

(fn PropelPlayer
  (bind _asbp_player (Utilities|Casting|CastToBP_Player (Components|GetOwner)))
  (|RespawnCheck _asbp_player)
  (bind _launchvelocity (CallFunction|GetLaunchVelocity (Variables|/Game/_EscapeVelocity/Characters/Player/BP_Player.BP_Player_C|GetGrounded _asbp_player) (Variables|/Game/_EscapeVelocity/Characters/Player/BP_Player.BP_Player_C|GetAimForward _asbp_player)))
  (Character|LaunchCharacter _asbp_player _launchvelocity false false)
  (Variables|Default|SetCooldownStarted true))

(fn SetPropulsionStrength
  (params (Strength :type Float%20%28double-precision%29))
  (Variables|Default|SetPropulsionStrength Strength))

(fn AngleCheck
  (params (CameraRotationZAxis :type Float%20%28double-precision%29))
  (bind _output_get (LocalVariables|SetZAxis CameraRotationZAxis))
  (if (and (> _output_get -6e+02) (< _output_get 9e+02))
    (Variables|Default|SetAngle "Normal")
    (elif (> (LocalVariables|GetZAxis) -6e+02)
      (Variables|Default|SetAngle "High")
      (elif (< (LocalVariables|GetZAxis) 9e+02)
        (Variables|Default|SetAngle "Low")))))

(fn ChargePropulsion
  (params (Seconds :type Float%20%28double-precision%29))
  (bind _output_get (LocalVariables|SetChargeTime Seconds))
  (CallFunction|SetPropulsionStrength (Math|Float|MapRangeClamped _output_get 0.0 2e+01 (Variables|Default|GetPropulsionStrength) (LocalVariables|GetChargeLevel3)))
  (Variables|Default|SetGlobalChargeLevel (* (LocalVariables|GetChargeTime) 2.0)))

(fn GetChargeLevel
  (bind _globalchargelevel (Variables|Default|GetGlobalChargeLevel))
  (if (>= _globalchargelevel 3.0)
    (return 3.0)
    (else
      (return _globalchargelevel))))

(fn GetLaunchVelocity
  (params (IsGrounded :type Boolean) (IsAimedForward :type Boolean))
  (LocalVariables|SetGrounded IsGrounded)
  (if IsAimedForward
    ;[0.01764 0.01764 0.01764] GetVelocityFromCameraRotation
    (bind _inverserotationforward (CallFunction|GetInverseCameraRotation))
    (bind _propulsionstrength (|ReducePropulsionOnGround))
    (bind _output_get (Variables|Default|SetVelocity (* _propulsionstrength _inverserotationforward)))
    (Variables|Default|SetCameraZAxis (.z _output_get))
    (else
      ;[0.01764 0.01764 0.01764] GetVelocityWhenFacingBackwards
      (bind _cameraforward (Camera|GetCameraRotation))
      (bind _propulsionstrength_2 (|ReducePropulsionOnGround_2))
      (bind _output_get_2 (Variables|Default|SetVelocity (* _propulsionstrength_2 _cameraforward)))
      (Variables|Default|SetCameraZAxis (.z _output_get_2))))
  (CallFunction|AngleCheck (Variables|Default|GetCameraZAxis)) ; Checking how much to increase z axis based on firing angle
  (return (Variables|Default|GetVelocity)))