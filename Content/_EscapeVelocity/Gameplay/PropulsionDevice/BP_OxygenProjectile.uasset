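; Oxygen projectile for the propulsion device that explodes on hit, launching the player and pushing physics objects.
; A sphere trace at impact launches the player away from the blast, with a boosted upward case for looking straight down.
; Other components receive impulses along projectile velocity; both pushes use distance math and the device's charge level.
; Global charge scales the explosion VFX, and the actor self-destroys after impact or a lifetime timeout.
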(event OnComponentHit(SphereCollider)
  (params (HitComponent :type Primitive%20Component%20Object%20Reference) (OtherActor :type Actor%20Object%20Reference) (OtherComp :type Primitive%20Component%20Object%20Reference) (NormalImpulse :type Vector :default "0, 0, 0") (Hit :type Hit%20Result%20Structure%20%28by%20ref%29))
  (bind (_returnvalue_z _playerupz) (|GetCameraRotationZ))
  (bind _spherecollider (Variables|Default|GetSphereCollider))
  (bind _spherecollider_2 (Variables|Default|GetSphereCollider))
  (bind _niagara (Variables|Default|GetNiagara))
  (bind _returnvalue (Transformation|GetWorldLocation _spherecollider))
  (bind _returnvalue_2 (Transformation|GetWorldLocation _spherecollider_2))
  (Variables|Default|SetImpact%20Point (.ImpactPoint (Collision|BreakHitResult Hit)))
  (bind _outhits (Collision|MultiSphereTraceByChannel _returnvalue _returnvalue 2.5e+02 "TraceTypeQuery3" false 0 "None" true "(R=1.000000,G=0.000000,B=0.000000,A=1.000000)" "(R=0.000000,G=1.000000,B=0.000000,A=1.000000)" 2.5))
  ;[0.01764 0.01764 0.01764] For Each hit component besides the player's collider add impulse
  (for _array_element _outhits
    (|MobiltyCheck (.HitComponent (Collision|BreakHitResult _array_element))) ; Checking if the hit component's mobility is set to moveable
    (if (== (Components|GetOwner (.HitComponent (Collision|BreakHitResult _array_element))) (Game|GetPlayerCharacter 0))
      ;[0.01764 0.01764 0.01764] Player Impulse Falloff Math
      (bind (_playerdirection _playerdistance) (CallFunction|CalculatePlayerDistance (Variables|Default|GetImpact%20Point)))
      (Variables|Default|SetPlayer%20Direction _playerdirection)
      (if (Math|Float|NearlyEqual(Float) _returnvalue_z _playerupz 1e-06)
        (Variables|Default|SetPlayer%20Direction (|UpwardsLaunch))
        (Variables|Default|SetPlayerImpulseStrength (Math|Conversions|ToFloat(Integer) (+ 15 (Math|Float|Round (Math|Float|MapRangeClamped 1e+02 0.0 _playerdistance 0.0 1e+01)))))
        (else
          (Variables|Default|SetPlayerImpulseStrength (Math|Conversions|ToFloat(Integer) (Math|Float|Round (Math|Float|MapRangeClamped 1e+02 0.0 _playerdistance 0.0 1e+01))))))
      ;[0.01764 0.01764 0.01764] PlayerLaunchVelocity
      (|ChargeImpulse) ; Increase Impulse By Charge Level
      (Character|LaunchCharacter (Game|GetPlayerCharacter 0) (* (Variables|Default|GetPlayer%20Direction) (Variables|Default|GetPlayerImpulseStrength)) false false)
      (else
        (|ChargePhysicsImpulse)
        (Physics|AddImpulseatLocation (.HitComponent (Collision|BreakHitResult _array_element)) (* (Variables|/Script/Engine.MovementComponent|GetVelocity (Variables|Default|GetProjectileMovement)) (|ImpulseFalloff (.HitComponent (Collision|BreakHitResult _array_element)))) (Variables|Default|GetImpact%20Point) "None"))))
  (Utilities|FlowControl|Sequence
    (:then_0
      (|GetGlobalCharge))
    (:then_1
      ;[0.01764 0.01764 0.01764] Play audio and vfx
      (|SetVFXTransform _niagara _returnvalue_2 (* (Variables|Default|GetExplosionScale) (Variables|Default|GetScalar)))
      (Components|Activation|Activate _niagara false)
      (Audio|PlaySoundatLocation "/Game/_EscapeVelocity/Sound/MetaSounds/MS_ProjectileExplosion.MS_ProjectileExplosion" _returnvalue_2 "0, 0, 0" 1.0 1.0 0.0 0 0 0 0)
      ;[0.01764 0.01764 0.01764] Hide projectile from player
      (Transformation|SetWorldScale3D (Variables|Default|GetOxygenProjectile) "0.001000,0.001000,0.001000")
      (|ChangeMobility))
    (:then_2
      ;[0.01764 0.01764 0.01764] Destroy Projectile
      (Utilities|FlowControl|Delay 2.0)
      (Actor|DestroyActor))))

(event Custom|OnExistedTooLong
  (Actor|DestroyActor))

(event EventBeginPlay
  (Utilities|Time|SetTimerbyEvent (EventDispatchers|CreateEvent :!event Custom|OnExistedTooLong) 5.0))

(event Collision|EventActorBeginOverlap
  (params (OtherActor :type Actor%20Object%20Reference)))

(event EventTick
  (params (DeltaSeconds :type Float%20%28single-precision%29)))

(fn ConstructionScript)

(fn CalculatePlayerDistance
  (params (Impact%20Point :type Vector))
  (bind _returnvalue (Game|GetPlayerCharacter 0))
  (bind _capsulecomponent (Variables|/Script/Engine.Character|GetCapsuleComponent _returnvalue))
  (bind _returnvalue_2 (Transformation|GetWorldLocation _capsulecomponent))
  (return (- _returnvalue_2 Impact%20Point) (Math|Vector|Distance(Vector) _returnvalue_2 Impact%20Point)))