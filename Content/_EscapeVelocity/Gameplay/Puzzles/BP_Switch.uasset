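; BP_Switch is a puzzle button that shows whether it is activated.
; On puzzle activation it reveals the ActivatedShader component and sinks the button mesh a short distance along its own up vector.
; Deactivation hides the component and raises the mesh by the same offset, with instant, unswept movement and no state check in this Blueprint.
; The shader component starts hidden on BeginPlay.
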(event EventBeginPlay
  (Rendering|SetVisibility (Variables|Default|GetActivatedShader) false false))

(event Collision|EventActorBeginOverlap
  (params (OtherActor :type Actor%20Object%20Reference)))

(event EventTick
  (params (DeltaSeconds :type Float%20%28single-precision%29)))

(event EventOnPuzzleActivate
  (bind _sm_structurebutton (Variables|Default|GetSM_StructureButton))
  ;[0.01764 0.01764 0.01764] ActivationColor
  (Rendering|SetVisibility (Variables|Default|GetActivatedShader) true false)
  (Transformation|AddWorldOffset _sm_structurebutton (* (Math|Vector|GetUpVector _sm_structurebutton) -1e+01) false false))

(event EventOnPuzzleDeactivate
  (bind _sm_structurebutton (Variables|Default|GetSM_StructureButton))
  ;[0.01764 0.01764 0.01764] ActivationColor
  (Rendering|SetVisibility (Variables|Default|GetActivatedShader) false false)
  (Transformation|AddWorldOffset _sm_structurebutton (* (Math|Vector|GetUpVector _sm_structurebutton) 1e+01) false false))

(fn ConstructionScript)