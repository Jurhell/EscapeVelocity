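; BP_ForceField is an obstacle that launches the player away from its center on hit until enough switches deactivate it.
; Entering the planet creates a switch-count widget, which updates on switch activation, while a counter tracks activations and deactivations against the trigger count.
; Reaching the count fades the widget, shows a HUD message and starts a looping timer that shrinks the field until it destroys itself.
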(event Custom|Deactivate
  (bind _returnvalue (Utilities|Time|SetTimerbyEvent (EventDispatchers|CreateEvent :!event Custom|OnShrink) 0.1 true true))
  (Variables|Default|SetForcefieldTimer _returnvalue)
  (bind _returnvalue_2 (UserInterface|CreateWidget "/Game/_EscapeVelocity/UI/WBP_HUDMessage.WBP_HUDMessage_C" (Game|GetPlayerController 0)))
  (Variables|/Game/_EscapeVelocity/UI/WBP_HUDMessage.WBP_HUDMessage_C|SetMessage _returnvalue_2 "Forcefield Deactivated")
  (UserInterface|Viewport|AddtoViewport _returnvalue_2 0)
  (Variables|Default|SetSwitchesActivated 0))

(event Custom|OnShrink
  (bind _returnvalue (Transformation|GetActorScale3D))
  (bind _shrinkspeed (Variables|Default|GetShrinkSpeed))
  (Transformation|SetActorScale3D (- (Transformation|GetActorScale3D) (Math|Vector|MakeVector _shrinkspeed _shrinkspeed _shrinkspeed)))
  (if (Math|Boolean|ORBoolean (< (.x _returnvalue) 0.0) (< (.y _returnvalue) 0.0) (< (.z _returnvalue) 0.0))
    (Utilities|Time|ClearandInvalidateTimerbyHandle (Variables|Default|GetForcefieldTimer))
    (Actor|DestroyActor)))

(event Custom|OnPlanetEnter
  (bind _returnvalue (UserInterface|CreateWidget "/Game/_EscapeVelocity/UI/WBP_SwitchCount.WBP_SwitchCount_C" (Game|GetPlayerController 0)))
  (UserInterface|Viewport|AddtoViewport _returnvalue 0)
  (Variables|Default|SetSwitchWidget _returnvalue))

(event Custom|OnSwitchActivated
  (bind _switchesactivated (Variables|Default|GetSwitchesActivated))
  (Math|Integer|IncrementInt _switchesactivated
    (:%20%20
      (if (>= _switchesactivated (Variables|Default|GetSwitchTriggerCount))
        (bind _switchwidget (Variables|Default|GetSwitchWidget)
          (:then
            (Default|BeginFade _switchwidget)
            (CallFunction|Deactivate))
          (:else)))
      (bind _switchwidget_2 (Variables|Default|GetSwitchWidget)
        (:then
          (Default|OnSwitchActivate _switchwidget_2))
        (:else)))))

(event Custom|OnSwitchDeactivated
  (Math|Integer|DecrementInt (Variables|Default|GetSwitchesActivated)))

(event Collision|EventHit
  (params (MyComp :type Primitive%20Component%20Object%20Reference) (Other :type Actor%20Object%20Reference) (OtherComp :type Primitive%20Component%20Object%20Reference) (bSelfMoved :type Boolean) (HitLocation :type Vector :default "0, 0, 0") (HitNormal :type Vector :default "0, 0, 0") (NormalImpulse :type Vector :default "0, 0, 0") (Hit :type Hit%20Result%20Structure%20%28by%20ref%29))
  (bind _asbp_player (Utilities|Casting|CastToBP_Player Other))
  (Character|LaunchCharacter _asbp_player (* (Math|Vector|GetUnitDirection(Vector) (Transformation|GetActorLocation) (Transformation|GetActorLocation Other)) (Variables|Default|GetLaunchStrength)) false false))

(fn ConstructionScript)