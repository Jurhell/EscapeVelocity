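; Base Blueprint for a destructible obstacle that breaks when an oxygen projectile overlaps it.
; On a hit it destroys the projectile, activates a Niagara effect and removes its static mesh, with a short timer to let the effect play before the actor is destroyed.
; The construction script sets CorrectRotation from RotateToGravity before running the parent construction script.
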(event Custom|OnEffectEnd
  (Actor|DestroyActor))

(event Collision|EventActorBeginOverlap
  (params (OtherActor :type Actor%20Object%20Reference))
  (bind _asbp_oxygen_projectile (Utilities|Casting|CastToBP_OxygenProjectile OtherActor))
  (Actor|DestroyActor _asbp_oxygen_projectile)
  (Components|Activation|Activate (Variables|Default|GetNiagara) false)
  (Components|DestroyComponent (Variables|Default|GetStaticMesh))
  (Utilities|Time|SetTimerbyEvent (EventDispatchers|CreateEvent :!event Custom|OnEffectEnd) 0.4))

(fn ConstructionScript
  (Variables|Default|SetCorrectRotation (Variables|Default|GetRotateToGravity))
  (|CallParentFunction))