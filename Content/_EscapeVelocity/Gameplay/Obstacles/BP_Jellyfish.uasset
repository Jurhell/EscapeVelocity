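; Jellyfish obstacle that can drain the player's oxygen and carries a launch pad as a child actor.
; DamageOxygen applies DamageAmount through player 0's BP_OxygenSystemComponent and stores that character; nothing in this file calls it.
; The construction script attaches the BP_LaunchPad child actor to TriggerBounds and shrinks its static mesh to a fixed world scale.
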(event EventBeginPlay)

(event Collision|EventActorBeginOverlap
  (params (OtherActor :type Actor%20Object%20Reference)))

(event EventTick
  (params (DeltaSeconds :type Float%20%28single-precision%29)))

(event EventDamageOxygen
  (bind _returnvalue (Game|GetPlayerCharacter 0))
  (Class|OxygenSystemComponent|TakeOxygenDamage (Actor|GetComponentbyClass _returnvalue "/Game/_EscapeVelocity/Gameplay/PropulsionDevice/BP_OxygenSystemComponent.BP_OxygenSystemComponent_C") (Variables|Default|GetDamageAmount))
  (Variables|Default|SetPlayerCharacter _returnvalue))

(fn ConstructionScript
  (Transformation|AttachComponentToComponent (Variables|Default|GetBP_LaunchPad) (Variables|Default|GetTriggerBounds) "None" "KeepRelative" "KeepRelative" "KeepRelative" true)
  (bind _asbp_launch_pad (Utilities|Casting|CastToBP_LaunchPad (Variables|/Script/Engine.ChildActorComponent|GetChildActor (Variables|Default|GetBP_LaunchPad))))
  (Transformation|SetWorldScale3D (Variables|/Game/_EscapeVelocity/Gameplay/Traversal/BP_LaunchPad.BP_LaunchPad_C|GetStaticMesh _asbp_launch_pad) "0.217500,0.217500,0.217500"))